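; Boid flock manager that spawns NumAgents BoidGpuBP actors at random points around SpawnLocation on BeginPlay.
; Once spawned, each boid receives the flock set, the manager as target, and the ID of its own MeshInstances instance.
; The manager then passes the flock to its own SetAll, targets itself and calls SetThinkGroups.
; Tick only applies a zero offset; instance-update and trace experiments are left unconnected.
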(event `self.ReceiveBeginPlay`
  (bind _boids (`self.Boids`))
  (bind _counter (`/Engine/EditorBlueprintResources/StandardMacros.Do N` (`self.NumAgents`) :!label _label)
    (:`Exit`
      (bind _returnvalue (`|SpawnActorFromClass` "/Game/BP/BoidGpuBP.BoidGpuBP_C" (`KismetMathLibrary.MakeTransform` (+ (`self.SpawnLocation`) (* (`KismetMathLibrary.RandomUnitVector`) (* (`KismetMathLibrary.RandomFloat`) (`self.SpawnArea`))))) "Undefined" "MultiplyWithRoot" null null))
      (`BlueprintSetLibrary.Set_Add` (`self.Boids`) _returnvalue)
      (if (>= _counter (`self.NumAgents`))
        (bind _result (`BlueprintSetLibrary.Set_ToArray` (`self.Boids`)))
        (for _array_element _result
          (`BoidGpu.SetAll` _array_element (`self.Boids`))
          (`BoidGpu.SetTarget` _array_element self)
          (bind _returnvalue_2 (`InstancedStaticMeshComponent.AddInstance` (`self.MeshInstances`) (`self.GetTransform` _array_element) true))
          (`KismetSystemLibrary.PrintString` (`KismetStringLibrary.Conv_IntToString` _returnvalue_2) false false)
          (`BoidGpu.SetId` _array_element _returnvalue_2))
        (`self.SetAll` _boids)
        (`KismetSystemLibrary.PrintText` (`KismetTextLibrary.Conv_IntToText` (`BlueprintSetLibrary.Set_Length` _boids)) false false)
        (`self.SetTarget` self)
        (`self.SetThinkGroups`)
        (else
          (goto _label))))))

(event `self.ReceiveTick`
  (params (DeltaSeconds :type "Float (single-precision)"))
  (`self.K2_SetActorLocation` (+ (`self.K2_GetActorLocation`) (0.0 0.0 0.0))))

(fn `UserConstructionScript`)